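; AI controller for the robot enemy that runs BT_Robot on possess and handles perception of the player.
; Sensing an actor tagged Player cancels the stop-chase timer and writes line-of-sight and the player reference to the Blackboard.
; Any other perception update, including losing the player or sensing a non-player, starts a one-shot LineOfSightTimer delay.
; When that delay expires, both Blackboard values are cleared.
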(event `self.ReceivePossess`
  (params (PossessedPawn :type "Pawn Object Reference"))
  (`self.RunBehaviorTree` "/Game/AI/Robot/BT_Robot.BT_Robot"))

(event `self.AIPerception.OnTargetPerceptionUpdated`
  (params (Actor :type "Actor Object Reference") (Stimulus :type "AIStimulus Structure"))
  (bind _blackboard (`self.Blackboard`))
  (if (and (`self.ActorHasTag` Actor "Player") (`.bSuccessfullySensed` (break `AIStimulus` Stimulus)))
    (`KismetSystemLibrary.K2_ClearAndInvalidateTimerHandle` (`self.StopChaseTimer`))
    (`BlackboardComponent.SetValueAsBool` _blackboard (`self.HasLineOfSight`) true)
    (`BlackboardComponent.SetValueAsObject` _blackboard (`self.APlayer`) Actor)
    (else
      (bind _returnvalue (`KismetSystemLibrary.K2_SetTimerDelegate` (delegate `StartStopChaseTimer`) (`self.LineOfSightTimer`)))
      (set `self.StopChaseTimer` _returnvalue))))

(event `StartStopChaseTimer`
  (bind _blackboard (`self.Blackboard`))
  (`BlackboardComponent.SetValueAsBool` _blackboard (`self.HasLineOfSight`) false)
  (`BlackboardComponent.SetValueAsObject` _blackboard (`self.APlayer`) null))

(fn `UserConstructionScript`)